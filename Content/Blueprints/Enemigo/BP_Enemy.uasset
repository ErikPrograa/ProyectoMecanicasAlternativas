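; Stationary-looking enemy that turns to face the player inside its PlayerDetection overlap and shoots fireballs at them.
; While the player is detected, Tick updates the look-at rotation and a DoOnce starts a looping Shoot timer on CoolDown.
; Shoot plays the Swarm attack montage, whose notify spawns BP_Fireball aimed at the player.
; Leaving the overlap clears the timer, and a second DoOnce triggers a timeline easing rotation back to zero.
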(event OnComponentBeginOverlap(PlayerDetection)
  (params (OverlappedComponent :type Primitive%20Component%20Object%20Reference) (OtherActor :type Actor%20Object%20Reference) (OtherComp :type Primitive%20Component%20Object%20Reference) (OtherBodyIndex :type Integer) (bFromSweep :type Boolean) (SweepResult :type Hit%20Result%20Structure%20%28by%20ref%29))
  ;[0.15 0.15 0.15 0.5] Collision events
  (if (Actor|ActorHasTag OtherActor "Player")
    (Variables|Default|SetPlayerDetected true)
    (Audio|Components|Audio|Stop (Variables|Default|GetTimelineLookAt0))))

(event OnComponentEndOverlap(PlayerDetection)
  (params (OverlappedComponent :type Primitive%20Component%20Object%20Reference) (OtherActor :type Actor%20Object%20Reference) (OtherComp :type Primitive%20Component%20Object%20Reference) (OtherBodyIndex :type Integer))
  ;[0.15 0.15 0.15 0.5] Collision events
  (if (Actor|ActorHasTag OtherActor "Player")
    (Variables|Default|SetPlayerDetected false)
    (Utilities|Time|ClearandInvalidateTimerbyHandle (Variables|Default|GetShootHandler))))

(event Custom|ReturnRotationToBase
  ;[0.15 0.15 0.15 0.5] Comment
  (Variables|Default|SetLastRotation (Transformation|GetActorRotation))
  (bind _alpha (Timeline|TimelineLookAt0 PlayFromStart)
    (:Update
      (Transformation|SetActorRotation (Math|Rotator|Lerp(Rotator) (Variables|Default|GetLastRotation) "0, 0, 0" _alpha)))
    (:Finished
      (Transformation|SetActorRotation "0, 0, 0"))))

(event Custom|Shoot
  ;[0.15 0.15 0.15 0.5] LookAtFunction
  (Animation|Montage|PlayMontage (Variables|Default|GetSkeletalMesh) "/Game/Characters/Models/AM_Swarm_Attack.AM_Swarm_Attack"
    (:OnNotifyBegin
      (Game|SpawnActorfromClass "/Game/Blueprints/Enemigo/BP_Fireball.BP_Fireball_C" (Math|Transform|MakeTransform (Transformation|GetActorLocation) "0, 0, 0" "1.000000,1.000000,1.000000") "Undefined" "MultiplyWithRoot" 0 (Math|Vector|GetForwardVector (Math|Rotator|FindLookatRotation (Transformation|GetActorLocation) (Transformation|GetActorLocation (Game|GetPlayerCharacter 0)))) 0))))

(event EventTick
  (params (DeltaSeconds :type Float%20%28single-precision%29))
  ;[0.15 0.15 0.15 0.5] LookAtFunction
  (if (Variables|Default|GetPlayerDetected)
    (Transformation|SetActorRotation (Math|Rotator|FindLookatRotation (Transformation|GetActorLocation) (Transformation|GetActorLocation (Game|GetPlayerCharacter 0))))
    (Utilities|FlowControl|Sequence
      (:then_0
        (Utilities|FlowControl|DoOnce false :!label _label
          (:Completed
            (if (not (Utilities|Time|IsValidTimerHandle (Variables|Default|GetShootHandler)))
              (bind _returnvalue (Utilities|Time|SetTimerbyFunctionName 0 "Shoot" (Variables|Default|GetCoolDown) true))
              (Variables|Default|SetShootHandler _returnvalue)))))
      (:then_1
        (goto _label_2 Reset)))
    (else
      (Utilities|FlowControl|Sequence
        (:then_0
          (Utilities|FlowControl|DoOnce true :!label _label_2
            (:Completed
              (CallFunction|ReturnRotationtoBase))))
        (:then_1
          (goto _label Reset))))))

(fn ConstructionScript)