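; BP_Fireball is an enemy projectile that knocks back characters it hits.
; The construction script copies its Velocity variable into ProjectileMovement.
; When its Sphere overlaps a Character, it launches that character with a strong push and slight lift, overriding current velocity, then destroys itself.
; The push direction always runs from the fireball toward player 0's character, whichever character was hit.
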(event OnComponentBeginOverlap(Sphere)
  (params (OverlappedComponent :type Primitive%20Component%20Object%20Reference) (OtherActor :type Actor%20Object%20Reference) (OtherComp :type Primitive%20Component%20Object%20Reference) (OtherBodyIndex :type Integer) (bFromSweep :type Boolean) (SweepResult :type Hit%20Result%20Structure%20%28by%20ref%29))
  (bind _ascharacter (Utilities|Casting|CastToCharacter OtherActor))
  (Character|LaunchCharacter _ascharacter (+ (* (Math|Vector|GetForwardVector (Math|Rotator|FindLookatRotation (Transformation|GetActorLocation) (Transformation|GetActorLocation (Game|GetPlayerCharacter 0)))) 1e+04) "0.000000,0.000000,100.000000") true true)
  (Actor|DestroyActor))

(fn ConstructionScript
  (Variables|/Script/Engine.MovementComponent|SetVelocity (Variables|Default|GetProjectileMovement) (Variables|Default|GetVelocity)))