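; BP_Scalable is an interactable prop that can be grown, shrunk, picked up and thrown, with its mesh set in the construction script.
; Interacting plays a timeline that lerps the uniform scale one step up or down within clamped limits, swapping material until it finishes and ignoring input meanwhile.
; Pickup attaches the mesh to the supplied parent, and Drop detaches it, enables physics and applies a velocity-change impulse.
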(event EventBeginPlay
  (Variables|Default|SetCurrentSize (.X (Math|Vector|BreakVector (Transformation|GetWorldScale (Variables|Default|GetCube))))))

(event EventPickup
  (params (Actor :type Scene%20Component%20Object%20Reference))
  (Transformation|AttachComponentToComponent (Variables|Default|GetCube) Actor "None" "SnapToTarget" "KeepRelative" "KeepRelative" true))

(event EventDrop
  (params (Impulse :type Vector :default "0, 0, 0"))
  (Transformation|DetachFromComponent (Variables|Default|GetCube) "KeepWorld" "KeepRelative" "KeepRelative" true)
  (Physics|SetSimulatePhysics (Variables|Default|GetCube) true)
  (Physics|AddImpulse (Variables|Default|GetCube) Impulse "None" true))

(event EventOnInteract
  (params (ScaleUp :type Boolean))
  (if (not (Audio|Components|Audio|IsPlaying (Variables|Default|GetScaleTimeLine)))
    (Rendering|Material|SetMaterial (Variables|Default|GetCube) 0 "/DatasmithContent/Materials/CE_OpaqueReference.CE_OpaqueReference")
    (if ScaleUp
      (Variables|Default|SetIncreaseValue 1.0)
      (bind _alpha (Timeline|ScaleTimeLine PlayFromStart)
        (:Update
          (Transformation|SetWorldScale3D (Variables|Default|GetCube) (Math|Conversions|ToVector(Float) (Math|Float|Lerp (Variables|Default|GetCurrentSize) (Math|Float|Clamp(Float) (+ (Variables|Default|GetCurrentSize) (Variables|Default|GetIncreaseValue)) 1.0 7.0) _alpha))))
        (:Finished
          (Variables|Default|SetCurrentSize (Math|Float|Clamp(Float) (+ (Variables|Default|GetCurrentSize) (Variables|Default|GetIncreaseValue)) 1.0 7.0))
          (Rendering|Material|SetMaterial (Variables|Default|GetCube) 0 "/Engine/BasicShapes/BasicShapeMaterial.BasicShapeMaterial")))
      (else
        (Variables|Default|SetIncreaseValue -1.0)
        (Timeline|ScaleTimeLine PlayFromStart)))))

(fn ConstructionScript
  (Components|StaticMesh|SetStaticMesh (Variables|Default|GetCube) (Variables|Default|GetStaticMesh)))