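; BP_MovingObjectCollectorZone is a puzzle zone that collects thrown gravity objects and rewards the player with a key.
; When a BP_ThrowGravityObject overlaps DetectionBox, the zone destroys it and increments a counter.
; Once three are collected, a one-time HasSpawned guard swaps ZoneMesh to the completed material and spawns BP_Key at the SpawnPoint transform.
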(event OnComponentBeginOverlap(DetectionBox)
  (params (OverlappedComponent :type Primitive%20Component%20Object%20Reference) (OtherActor :type Actor%20Object%20Reference) (OtherComp :type Primitive%20Component%20Object%20Reference) (OtherBodyIndex :type Integer) (bFromSweep :type Boolean) (SweepResult :type Hit%20Result%20Structure%20%28by%20ref%29))
  (bind _asbp_throw_gravity_object (Utilities|Casting|CastToBP_ThrowGravityObject OtherActor))
  (Actor|DestroyActor _asbp_throw_gravity_object)
  (Variables|Default|SetDestroyedCount (+ (Variables|Default|GetDestroyedCount) 1))
  (if (>= (Variables|Default|GetDestroyedCount) 3)
    (if (== (Variables|Default|GetHasSpawned) false)
      (Variables|Default|SetHasSpawned true)
      (Rendering|Material|SetMaterial (Variables|Default|GetZoneMesh) 0 (Variables|Default|GetCompletetMaterial))
      (Game|SpawnActorfromClass "/Game/Blueprints/Interactuables/BP_Key.BP_Key_C" (Transformation|GetActorTransform (Variables|Default|GetSpawnPoint)) "Undefined" "MultiplyWithRoot" 0 1 0))))

(event EventBeginPlay)

(event Collision|EventActorBeginOverlap
  (params (OtherActor :type Actor%20Object%20Reference)))

(event EventTick
  (params (DeltaSeconds :type Float%20%28single-precision%29)))

(fn ConstructionScript)