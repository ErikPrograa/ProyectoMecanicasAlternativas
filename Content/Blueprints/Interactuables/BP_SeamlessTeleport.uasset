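; Seamless teleporter that moves the player from an Entrance box to an Exit box without breaking their motion.
; When any Character overlaps Entrance, player 0's transform, velocity and control rotation are re-expressed relative to the exit.
; Transform and velocity use the box components as reference frames, while view direction uses EntranceFwd and ExitFwd.
; The construction script sizes both boxes from a shared BoxSize.
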(event OnComponentBeginOverlap(Entrance)
  (params (OverlappedComponent :type Primitive%20Component%20Object%20Reference) (OtherActor :type Actor%20Object%20Reference) (OtherComp :type Primitive%20Component%20Object%20Reference) (OtherBodyIndex :type Integer) (bFromSweep :type Boolean) (SweepResult :type Hit%20Result%20Structure%20%28by%20ref%29))
  ;[0.15 0.15 0.15 0.5] Character edit
  (Utilities|Casting|CastToCharacter OtherActor)
  (Transformation|SetActorTransform (Game|GetPlayerCharacter 0) (CallFunction|GetDestinationTransform))
  (Variables|/Script/Engine.MovementComponent|SetVelocity (Pawn|GetMovementComponent (Game|GetPlayerCharacter 0)) (CallFunction|GetNewVelocity))
  ;[0.15 0.15 0.15 0.5] Controller Edit
  (Pawn|SetControlRotation (Game|GetPlayerController 0) (CallFunction|GetNewControlRotation)))

(fn ConstructionScript
  (Components|Box|SetBoxExtent (Variables|Default|GetEntrance) (Variables|Default|GetBoxSize) true))

(fn GetDestinationTransform
  (return (Math|Transform|ComposeTransforms (Math|Transform|MakeRelativeTransform (Transformation|GetActorTransform (Game|GetPlayerCharacter 0)) (Transformation|GetWorldTransform (Variables|Default|GetEntrance))) (Transformation|GetWorldTransform (Variables|Default|GetExit)))))

(fn GetNewControlRotation
  (return (Math|Rotator|MakeRotfromX (Math|Vector|RotateVector (Math|Vector|UnrotateVector (Math|Vector|GetForwardVector (Pawn|GetControlRotation (Game|GetPlayerCharacter 0) :!class /Script/Engine.Pawn)) (Transformation|GetWorldRotation (Variables|Default|GetEntranceFwd))) (Transformation|GetWorldRotation (Variables|Default|GetExitFwd))))))

(fn GetNewVelocity
  (return (Math|Vector|RotateVector (Math|Vector|UnrotateVector (Variables|/Script/Engine.MovementComponent|GetVelocity (Pawn|GetMovementComponent (Game|GetPlayerCharacter 0))) (Transformation|GetWorldRotation (Variables|Default|GetEntrance))) (Transformation|GetWorldRotation (Variables|Default|GetExit)))))