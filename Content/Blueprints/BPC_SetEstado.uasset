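; BPC_SetEstado is a Blueprint that switches a target mesh between ghost and solid states by Gameplay Tag.
; Its EstadoNuevo event validates the tag, stores it with the target, then switches on it.
; Estado.Fantasma applies a transparent material and overlaps every channel except Visibility, which still blocks.
; Estado.Solido blocks all channels and applies a prototype grid material.
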(event Custom|EstadoNuevo
  (params (GameplayTag :type Gameplay%20Tag%20Structure) (Target :type Primitive%20Component%20Object%20Reference))
  (if (GameplayTags|IsGameplayTagValid GameplayTag)
    (Variables|Default|SetMeshToChange Target)
    (Variables|Default|SetTag GameplayTag)
    (|SwitchGameplayTag (Variables|Default|GetTag)
      (:Estado.Fantasma
        (Collision|SetCollisionResponsetoAllChannels (Variables|Default|GetMeshToChange) "ECR_Overlap")
        (Rendering|Material|SetMaterial (Variables|Default|GetMeshToChange) 0 "/Game/Blueprints/Materiales/M_Transparent.M_Transparent")
        (Collision|SetCollisionResponsetoChannel (Variables|Default|GetMeshToChange) "ECC_Visibility" "ECR_Block"))
      (:Estado.Solido
        (Collision|SetCollisionResponsetoAllChannels (Variables|Default|GetMeshToChange) "ECR_Block")
        (Rendering|Material|SetMaterial (Variables|Default|GetMeshToChange) 0 "/Game/LevelPrototyping/Materials/MI_PrototypeGrid_TopDark.MI_PrototypeGrid_TopDark")))))