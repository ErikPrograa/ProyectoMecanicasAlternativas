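; Timed scalable platform that grows or shrinks horizontally when interacted with, then returns to its original size.
; OnInteract plays a timeline that lerps the cube's X/Y scale by a clamped step at fixed thickness, ignoring input while playing.
; When off its original size, a retriggerable delay precedes a material swap and a replay of the timeline back to that size.
; Pickup and Drop events are empty, with their attach and physics logic left unconnected.
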(event EventBeginPlay
  (bind _cube (Variables|Default|GetCube))
  (bind _returnvalue (Transformation|GetWorldScale _cube))
  (bind _x (Math|Vector|BreakVector _returnvalue))
  (Variables|Default|SetCurrentSize _x)
  (Variables|Default|SetOriginalSize _x))

(event EventPickup
  (params (Actor :type Scene%20Component%20Object%20Reference)))

(event EventDrop
  (params (Impulse :type Vector :default "0, 0, 0")))

(event EventOnInteract
  (params (ScaleUp :type Boolean))
  (if (not (Audio|Components|Audio|IsPlaying (Variables|Default|GetScaleTimeLine)))
    (Rendering|Material|SetMaterial (Variables|Default|GetCube) 0 "/DatasmithContent/Materials/CE_OpaqueReference.CE_OpaqueReference")
    (if ScaleUp
      (Variables|Default|SetIncreaseValue 3.0)
      (bind _alpha (Timeline|ScaleTimeLine PlayFromStart)
        (:Update
          (Transformation|SetWorldScale3D (Variables|Default|GetCube) (Math|Vector|MakeVector (Math|Float|Lerp (Variables|Default|GetCurrentSize) (Math|Float|Clamp(Float) (+ (Variables|Default|GetCurrentSize) (Variables|Default|GetIncreaseValue)) 1.0 13.0) _alpha) (Math|Float|Lerp (Variables|Default|GetCurrentSize) (Math|Float|Clamp(Float) (+ (Variables|Default|GetCurrentSize) (Variables|Default|GetIncreaseValue)) 1.0 13.0) _alpha) 0.05)))
        (:Finished
          (Variables|Default|SetCurrentSize (Math|Float|Clamp(Float) (+ (Variables|Default|GetCurrentSize) (Variables|Default|GetIncreaseValue)) 1.0 13.0))
          (if (not (Math|Float|NearlyEqual(Float) (Variables|Default|GetCurrentSize) (Variables|Default|GetOriginalSize) 0.01))
            (Utilities|FlowControl|RetriggerableDelay 1.0)
            (Variables|Default|SetIncreaseValue (- (Variables|Default|GetOriginalSize) (Variables|Default|GetCurrentSize)))
            (Rendering|Material|SetMaterial (Variables|Default|GetCube) 0 "/Engine/VREditor/BasicMeshes/MI_Cube_03.MI_Cube_03")
            (Timeline|ScaleTimeLine PlayFromStart))))
      (else
        (Variables|Default|SetIncreaseValue -3.0)
        (Timeline|ScaleTimeLine PlayFromStart)))))

(fn ConstructionScript
  (Components|StaticMesh|SetStaticMesh (Variables|Default|GetCube) (Variables|Default|GetStaticMesh)))