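; BP_GravityObject is an interactable object whose static mesh loses gravity and launches upward when used.
; On the first OnInteract only, it disables gravity, applies a mass-independent upward velocity impulse and adds a random rotation.
; A separate FloatMesh function does the same to a passed-in target with a weaker impulse, but nothing in this Blueprint calls it.
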(event EventOnInteract
  (params (ScaleUp :type Boolean))
  (Utilities|FlowControl|DoOnce false
    (:Completed
      (Physics|SetEnableGravity (Variables|Default|GetStaticMesh) false)
      (Physics|AddImpulse (Variables|Default|GetStaticMesh) "0.000000,0.000000,400.000000" "None" true)
      (Transformation|AddWorldRotation (Variables|Default|GetStaticMesh) (Math|Random|RandomRotator true) false false))))

(fn ConstructionScript)

(fn FloatMesh
  (params (Target123 :type Primitive%20Component%20Object%20Reference))
  (Physics|SetEnableGravity Target123 false)
  (Physics|AddImpulse Target123 "0.000000,0.000000,100.000000" "None" true)
  (Transformation|AddWorldRotation Target123 (Math|Random|RandomRotator true) false false))