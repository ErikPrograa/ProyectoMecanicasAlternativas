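; Throwable physics prop that can be floated, picked up and thrown.
; Its first interaction disables gravity on the static mesh, launches it upward and tilts it once.
; Pickup snaps the mesh to the supplied parent; Drop detaches it, simulates physics and applies a scaled velocity impulse with zero linear damping, without restoring gravity.
; A separate FloatMesh function similarly lifts a target with random rotation, but nothing here calls it.
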(event EventPickup
  (params (Actor :type Scene%20Component%20Object%20Reference))
  (Transformation|AttachComponentToComponent (Variables|Default|GetStaticMesh) Actor "None" "SnapToTarget" "KeepRelative" "KeepRelative" true))

(event EventDrop
  (params (Impulse :type Vector :default "0, 0, 0"))
  (Transformation|DetachFromComponent (Variables|Default|GetStaticMesh) "KeepWorld" "KeepRelative" "KeepRelative" true)
  (Physics|SetSimulatePhysics (Variables|Default|GetStaticMesh) true)
  (Physics|AddImpulse (Variables|Default|GetStaticMesh) (* Impulse "20.000000,20.000000,20.000000") "None" true)
  (Class|PrimitiveComponent|SetLinearDamping (Variables|Default|GetStaticMesh) 0.0))

(event EventOnInteract
  (params (ScaleUp :type Boolean))
  (Utilities|FlowControl|DoOnce false
    (:Completed
      (Physics|SetEnableGravity (Variables|Default|GetStaticMesh) false)
      (Physics|AddImpulse (Variables|Default|GetStaticMesh) "0.000000,0.000000,450.000000" "None" true)
      (Transformation|AddWorldRotation (Variables|Default|GetStaticMesh) (Math|Rotator|MakeRotator 1e+01 0.0 25.0) false false))))

(fn ConstructionScript)

(fn FloatMesh
  (params (Target123 :type Primitive%20Component%20Object%20Reference))
  (Physics|SetEnableGravity Target123 false)
  (Physics|AddImpulse Target123 "0.000000,0.000000,100.000000" "None" true)
  (Transformation|AddWorldRotation Target123 (Math|Random|RandomRotator true) false false))